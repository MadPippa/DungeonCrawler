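; BP_BubbleGun is a player bubble gun actor that blows and releases bubbles.
; BeginBubbleBlow spawns an actor of PotionClass at its Arrow component, stores it as Bubble, attaches it there and tells it to begin blowing.
; EndBubbleBlow detaches a valid Bubble, keeping its world transform, and tells it to end blowing, leaving the blowing behavior to the spawned actor.
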(event Custom|BeginBubbleBlow
  (bind _returnvalue (Game|SpawnActorfromClass (Variables|Default|GetPotionClass) (Transformation|GetWorldTransform (Variables|Default|GetArrow)) "Undefined" "MultiplyWithRoot" 0 0))
  (bind _output_get (Variables|Default|SetBubble _returnvalue))
  (Transformation|AttachComponentToComponent _output_get (Variables|Default|GetArrow) "None" "SnapToTarget" "SnapToTarget" "SnapToTarget" true)
  (Default|BeginBlowing _output_get))

(event Custom|EndBubbleBlow
  (bind _bubble (Variables|Default|GetBubble)
    (:then
      (Transformation|DetachFromActor _bubble "KeepWorld" "KeepWorld" "KeepWorld")
      (Default|EndBlowing _bubble))
    (:else)))

(event EventBeginPlay)

(event Collision|EventActorBeginOverlap
  (params (OtherActor :type Actor%20Object%20Reference)))

(event EventTick
  (params (DeltaSeconds :type Float%20%28single-precision%29)))

(fn ConstructionScript)