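; BP_Potion_Base is a base potion projectile that is blown up like a bubble, then fired, with splash effects on impact.
; A looping timer grows BubblePower while blowing, bursting the bubble at maximum.
; On release, low power destroys it; otherwise projectile movement launches it forward at FirePower.
; Non-ignored hits trigger a sphere trace, passing each hit actor to the empty PotionEffect hook before self-destructing.
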(event Custom|PotionEffect
  (params (HitActor :type Actor%20Object%20Reference)))

(event Custom|BeginBlowing
  (Utilities|Time|SetTimerbyFunctionName 0 "BlowTick" (Variables|Default|GetBlowTickFreq) true))

(event Custom|EndBlowing
  (Utilities|Time|ClearTimerbyFunctionName 0 "BlowTick")
  (if (<= (Variables|Default|GetBubblePower) (Variables|Default|GetRoundDownPoint))
    (CallFunction|UnBlowBubble)
    (else
      (CallFunction|FireBubble))))

(event Custom|BubbleBurst
  (Development|PrintString "Burst")
  (Actor|DestroyActor))

(event Custom|UnBlowBubble
  (Development|PrintString "UnBlow")
  (Actor|DestroyActor))

(event Custom|FireBubble
  (bind _projectilemovement (Variables|MyProjectile|GetProjectileMovement))
  (Development|PrintString "FireBubble")
  (Components|Activation|Activate _projectilemovement true)
  (Variables|/Script/Engine.ProjectileMovementComponent|SetInitialSpeed _projectilemovement 3e+03)
  (Variables|/Script/Engine.ProjectileMovementComponent|SetMaxSpeed _projectilemovement 3e+03)
  (Variables|/Script/Engine.MovementComponent|SetVelocity _projectilemovement (* (Transformation|GetActorForwardVector) (Variables|Default|GetFirePower))))

(event EventBeginPlay
  (Components|Activation|Deactivate (Variables|MyProjectile|GetProjectileMovement)))

(event Collision|EventHit
  (params (MyComp :type Primitive%20Component%20Object%20Reference) (Other :type Actor%20Object%20Reference) (OtherComp :type Primitive%20Component%20Object%20Reference) (bSelfMoved :type Boolean) (HitLocation :type Vector :default "0, 0, 0") (HitNormal :type Vector :default "0, 0, 0") (NormalImpulse :type Vector :default "0, 0, 0") (Hit :type Hit%20Result%20Structure%20%28by%20ref%29))
  (if (not (Utilities|Array|ContainsItem (Variables|Default|GetIgnoreHitClasses) (Utilities|GetClass Other)))
    (bind _outhits (Collision|MultiSphereTraceByChannel HitLocation HitLocation (Variables|Default|GetSplashRadius) "TraceTypeQuery1" false 0 "None"))
    (for _array_element _outhits
      (CallFunction|PotionEffect (.HitActor (Collision|BreakHitResult _array_element))))
    (Actor|DestroyActor) ; Then destroy this projectile
  ))

(fn ConstructionScript)

(fn BlowTick
  (bind _output_get (Variables|Default|SetBubblePower (Math|Float|Lerp 0.0 1e+02 (/ (Variables|Default|GetCurrentBlowTickTime) (Variables|Default|GetMaxBlowTickTime)))))
  (if (>= _output_get 1e+02)
    (CallFunction|BubbleBurst)
    (else
      (if (>= _output_get (Variables|Default|GetRoundUpPoint))
        (Variables|Default|SetBubblePower 1e+02))
      (Variables|Default|SetCurrentBlowTickTime (+ (Variables|Default|GetBlowTickFreq) (Variables|Default|GetCurrentBlowTickTime))))))