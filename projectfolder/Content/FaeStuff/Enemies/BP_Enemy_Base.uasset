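; Base enemy Blueprint that supplies AI setup, melee attacks and removal for enemy characters.
; On BeginPlay it passes AI info, patrol paths and target classes to its controller and creates a dynamic mesh material.
; A collision component tracks target-class actors in range, updates a Blackboard flag, and MeleeAttack damages their health components.
; Death destroys it immediately, BeginDisappear fades opacity before destroying it, and GetNextPatrolPoint is an empty stub.
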(event OnComponentBeginOverlap(MeleeAttackCollision)
  (params (OverlappedComponent :type Primitive%20Component%20Object%20Reference) (OtherActor :type Actor%20Object%20Reference) (OtherComp :type Primitive%20Component%20Object%20Reference) (OtherBodyIndex :type Integer) (bFromSweep :type Boolean) (SweepResult :type Hit%20Result%20Structure%20%28by%20ref%29))
  (if (Utilities|Array|ContainsItem (Variables|Default|GetTargetClasses) (Utilities|GetClass OtherActor))
    (Utilities|Array|AddUnique (Variables|Default|GetTargetsInMelee) OtherActor)
    (CallFunction|UpdateTargetsinMelee)))

(event OnComponentEndOverlap(MeleeAttackCollision)
  (params (OverlappedComponent :type Primitive%20Component%20Object%20Reference) (OtherActor :type Actor%20Object%20Reference) (OtherComp :type Primitive%20Component%20Object%20Reference) (OtherBodyIndex :type Integer))
  (if (Utilities|Array|ContainsItem (Variables|Default|GetTargetClasses) (Utilities|GetClass OtherActor))
    (Utilities|Array|RemoveItem (Variables|Default|GetTargetsInMelee) OtherActor)
    (CallFunction|UpdateTargetsinMelee)))

(event EventBeginPlay
  (bind _returnvalue (Pawn|GetController))
  (bind _mesh (Variables|Character|GetMesh))
  (Class|BIAIInfo|SetEnemyInfo(Message) _returnvalue (Variables|Default|GetAIInfo))
  (Class|BIAIInfo|SetPatrolPaths(Message) _returnvalue (Variables|Default|GetPatrolPaths))
  (Class|BIAIInfo|SetTargetClasses(Message) _returnvalue (Variables|Default|GetTargetClasses))
  (bind _returnvalue_2 (Rendering|Material|CreateDynamicMaterialInstance (Rendering|Material|GetMaterial _mesh 0) "None" "None" :!class /Script/Engine.KismetMaterialLibrary))
  (Variables|Default|SetMaterialInstance _returnvalue_2)
  (Rendering|Material|SetMaterial _mesh 0 _returnvalue_2))

(event EventMeleeAttack
  (for _array_element (Variables|Default|GetTargetsInMelee)
    (Utilities|IsValid (Actor|GetComponentbyClass _array_element "/Game/FaeStuff/Health/AC_Health.AC_Health_C")
      (:Is%20Valid
        (Class|BIHealth|Damage(Message) (Actor|GetComponentbyClass _array_element "/Game/FaeStuff/Health/AC_Health.AC_Health_C") (Variables|Default|GetDamageAmount))))))

(event EventBeginDisappear
  (bind _newtrack_0 (Timeline|DisappearTimeline Play)
    (:Update
      (Rendering|Material|SetScalarParameterValue (stale EventBeginPlay _returnvalue_2) "Opacity" (- 1.0 _newtrack_0) :!class /Script/Engine.MaterialInstanceDynamic))
    (:Finished
      (Actor|DestroyActor))))

(event EventDeath
  (Actor|DestroyActor))

(fn ConstructionScript)

(fn UpdateTargetsinMelee
  (bind _returnvalue (AI|GetBlackboard 0))
  (Utilities|IsValid _returnvalue
    (:Is%20Valid
      (AI|Components|Blackboard|SetValueasBool _returnvalue (Utilities|Name|MakeLiteralName "TargetsInMelee?") (Utilities|Array|IsNotEmpty (Variables|Default|GetTargetsInMelee))))))

(fn GetNextPatrolPoint
  (return 0))