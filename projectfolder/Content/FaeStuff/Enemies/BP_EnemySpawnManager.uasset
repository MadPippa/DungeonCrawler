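; BP_EnemySpawnManager is a manager actor that populates the level with zombies when play begins.
; On BeginPlay it caches every BP_ZombieSpawnLocation in the level and runs SpawnZombies.
; That event has each location remove its old zombie, then rolls the location's SpawnChance as a weighted random bool to decide whether it spawns a new one.
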(event Custom|SpawnZombies
  (for _array_element (Variables|Default|GetZombieSpawnLocations)
    (Default|RemoveOldZombie _array_element)
    (if (Math|Random|RandomBoolwithWeight (Variables|/Game/FaeStuff/Blueprints/Enemies/BP_ZombieSpawnLocation.BP_ZombieSpawnLocation_C|GetSpawnChance _array_element))
      (Default|SpawnZombie _array_element)
      (Development|PrintString "ShouldSpawn"))))

(event EventBeginPlay
  (bind _outactors (Actor|GetAllActorsOfClass "/Game/FaeStuff/Blueprints/Enemies/BP_ZombieSpawnLocation.BP_ZombieSpawnLocation_C"))
  (Variables|Default|SetZombieSpawnLocations _outactors)
  (CallFunction|SpawnZombies))

(event Collision|EventActorBeginOverlap
  (params (OtherActor :type Actor%20Object%20Reference)))

(event EventTick
  (params (DeltaSeconds :type Float%20%28single-precision%29)))

(fn ConstructionScript)