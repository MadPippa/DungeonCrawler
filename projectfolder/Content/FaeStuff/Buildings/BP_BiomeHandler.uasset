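; BP_BiomeHandler sets the active biome and broadcasts it to biome-aware actors.
; SetBiome stores the biome, then sends UpdateBiomeMessage to every actor implementing BI_BiomeInterface.
; The Construction Script applies the configured Biome, so changes propagate at edit time.
; BeginPlay replaces it with a random pick from PotentialBiomes.
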(event Custom|SetBiome
  (params (Biome :type E_Biome%20Enum :default "NewEnumerator0"))
  (bind _output_get (Variables|Default|SetBiome Biome))
  (bind _outactors (Actor|GetAllActorswithInterface "/Game/FaeStuff/Buildings/BI_BiomeInterface.BI_BiomeInterface_C"))
  (for _array_element _outactors
    (Class|BIBiomeInterface|UpdateBiome(Message) _array_element _output_get)))

(event EventBeginPlay
  (CallFunction|SetBiome (.OutItem (Utilities|Array|Random (Variables|Default|GetPotentialBiomes)))))

(fn ConstructionScript
  (CallFunction|SetBiome (Variables|Default|GetBiome)))