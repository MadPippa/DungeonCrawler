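; BP_Building_Base is a building Blueprint, apparently meant as a base, whose static mesh varies by biome.
; UpdateMesh selects the Castle, Hedge or Palisade mesh from the Biome value and applies it to the StaticMesh component.
; The construction script calls UpdateMesh, and the UpdateBiome event stores a new biome and refreshes the mesh.
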(event EventBeginPlay)

(event Collision|EventActorBeginOverlap
  (params (OtherActor :type Actor%20Object%20Reference)))

(event EventTick
  (params (DeltaSeconds :type Float%20%28single-precision%29)))

(event EventUpdateBiome
  (params (Biome :type E_Biome%20Enum :default "NewEnumerator0"))
  (Variables|Default|SetBiome Biome)
  (CallFunction|UpdateMesh))

(fn ConstructionScript
  (CallFunction|UpdateMesh))

(fn UpdateMesh
  (Components|StaticMesh|SetStaticMesh (Variables|Default|GetStaticMesh) (Utilities|Select :Index (Variables|Default|GetBiome) :NewEnumerator0 (Variables|Default|GetCastleMesh) :NewEnumerator1 (Variables|Default|GetHedgeMesh) :NewEnumerator2 (Variables|Default|GetPalisadeMesh))))