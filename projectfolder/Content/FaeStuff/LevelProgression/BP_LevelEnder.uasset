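; BP_LevelEnder is a hold-to-interact object that advances to the next level through BP_SaveManager.
; BeginInteract resets progress and starts a looping InteractTick timer, which accumulates time with PerTickTimer and calls StopTrying when maxed out.
; EndInteract clears the timer and passes MaxInteractTimer >= CurrentInteractTimer as success, so releasing before the maximum also succeeds.
; StopTrying calls NextLevel on the save manager cached at BeginPlay when successful.
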(event Custom|StopTrying
  (params (Succeeded? :type Boolean))
  (if Succeeded?
    (Default|NextLevel (Variables|Default|GetSaveManager))))

(event EventBeginPlay
  (bind _returnvalue (Actor|GetActorOfClass "/Game/FaeStuff/Save/BP_SaveManager.BP_SaveManager_C"))
  (Variables|Default|SetSaveManager _returnvalue))

(event EventBeginInteract
  (Variables|Default|SetCurrentInteractTimer 0.0)
  (Utilities|Time|SetTimerbyFunctionName 0 "InteractTick" (Variables|Default|GetInteractTickTime) true))

(event EventEndInteract
  (Utilities|Time|ClearTimerbyFunctionName 0 "InteractTick")
  (CallFunction|StopTrying (>= (Variables|Default|GetMaxInteractTimer) (Variables|Default|GetCurrentInteractTimer))))

(fn ConstructionScript)

(fn InteractTick
  (bind (_maxxedout_ _current_tick) (CallFunction|PerTickTimer (Variables|Default|GetMaxInteractTimer) 0.0 (Variables|Default|GetInteractTickTime) (Variables|Default|GetCurrentInteractTimer)))
  (Variables|Default|SetCurrentInteractTimer _current_tick)
  (if _maxxedout_
    (Utilities|Time|ClearTimerbyFunctionName 0 "InteractTick")
    (CallFunction|StopTrying _maxxedout_)))