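; BP_DCCharacter is the first-person player character, handling Enhanced Input movement, look, jump, bubble-gun shooting and interaction.
; On BeginPlay it attaches the BubbleGun child actor to the mesh's grip socket and caches the save manager.
; Looking, moving and interacting refresh a camera-forward sphere trace that adds its first hit to a never-cleared candidate array.
; The candidate nearest the player receives begin and end interact messages.
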(event Input|EnhancedActionEvents|EnhancedInputActionIA_DCShoot
  (params (ActionValue :type Boolean) (ElapsedSeconds :type Float%20%28double-precision%29) (TriggeredSeconds :type Float%20%28double-precision%29) (InputAction :type Input%20Action%20Object%20Reference :default "/Game/FaeStuff/Player/Controls/IA_DCShoot.IA_DCShoot"))
  (bind _weapon (Variables|Default|GetWeapon))
  (:Started
    (Default|BeginBubbleBlow _weapon))
  (:Canceled
    (Default|EndBubbleBlow _weapon :!label _label))
  (:Completed
    (goto _label)))

(event Input|EnhancedActionEvents|EnhancedInputActionIA_DCLook
  (params (ActionValue :type Vector%202D%20Structure) (ElapsedSeconds :type Float%20%28double-precision%29) (TriggeredSeconds :type Float%20%28double-precision%29) (InputAction :type Input%20Action%20Object%20Reference :default "/Game/FaeStuff/Player/Controls/IA_DCLook.IA_DCLook"))
  (Pawn|Input|AddControllerYawInput (.x ActionValue))
  (Pawn|Input|AddControllerPitchInput (.y ActionValue))
  (CallFunction|UpdateClosestInteract))

(event Input|EnhancedActionEvents|EnhancedInputActionIA_DCInteract
  (params (ActionValue :type Boolean) (ElapsedSeconds :type Float%20%28double-precision%29) (TriggeredSeconds :type Float%20%28double-precision%29) (InputAction :type Input%20Action%20Object%20Reference :default "/Game/FaeStuff/Player/Controls/IA_DCInteract.IA_DCInteract"))
  (bind _closestinteractable (Variables|Default|GetClosestInteractable))
  (:Started
    (CallFunction|UpdateClosestInteract)
    (Class|BIInteract|BeginInteract(Message) _closestinteractable))
  (:Canceled
    (Class|BIInteract|EndInteract(Message) _closestinteractable :!label _label)
    (CallFunction|UpdateClosestInteract))
  (:Completed
    (goto _label)))

(event Input|EnhancedActionEvents|EnhancedInputActionIA_DCMove
  (params (ActionValue :type Vector%202D%20Structure) (ElapsedSeconds :type Float%20%28double-precision%29) (TriggeredSeconds :type Float%20%28double-precision%29) (InputAction :type Input%20Action%20Object%20Reference :default "/Game/FaeStuff/Player/Controls/IA_DCMove.IA_DCMove"))
  (Pawn|Input|AddMovementInput (Transformation|GetActorRightVector) (.x ActionValue) false)
  (Pawn|Input|AddMovementInput (Transformation|GetActorForwardVector) (.y ActionValue) false)
  (CallFunction|UpdateClosestInteract))

(event Input|EnhancedActionEvents|EnhancedInputActionIA_DCJump
  (params (ActionValue :type Boolean) (ElapsedSeconds :type Float%20%28double-precision%29) (TriggeredSeconds :type Float%20%28double-precision%29) (InputAction :type Input%20Action%20Object%20Reference :default "/Game/FaeStuff/Player/Controls/IA_DCJump.IA_DCJump"))
  (:Started
    (Character|Jump))
  (:Canceled
    (Character|StopJumping :!label _label))
  (:Completed
    (goto _label)))

(event EventBeginPlay
  (Variables|Default|SetWeapon (.AsBP%20Bubble%20Gun (Utilities|Casting|CastToBP_BubbleGun (Variables|/Script/Engine.ChildActorComponent|GetChildActor (Variables|Default|GetBubbleGun)))))
  (Transformation|AttachComponentToComponent (Variables|Default|GetBubbleGun) (Variables|Default|GetFirstPersonMesh) "GripPoint" "SnapToTarget" "SnapToTarget" "SnapToTarget" true)
  (bind _returnvalue (Actor|GetActorOfClass "/Game/FaeStuff/Save/BP_SaveManager.BP_SaveManager_C"))
  (Variables|Default|SetSaveManager _returnvalue))

(fn ConstructionScript)

(fn UpdateClosestInteract
  (bind _returnvalue (Game|GetPlayerCameraManager 0))
  (bind _returnvalue_2 (Transformation|GetActorLocation _returnvalue))
  (bind _outhits (Collision|MultiSphereTraceByChannel _returnvalue_2 (+ _returnvalue_2 (* (Transformation|GetActorForwardVector _returnvalue) (Variables|Default|GetInteractRange))) (Variables|Default|GetInteractForgiveness) "TraceTypeQuery1" false 0 "ForOneFrame"))
  (bind _array_element (Utilities|Array|ForEachLoopwithBreak _outhits :!label _label)
    (:LoopBody
      (Utilities|Array|AddUnique (Variables|Default|GetInteractablesInInteract) (.HitActor (Collision|BreakHitResult _array_element)))
      (goto _label Break))
    (:Completed
      (Variables|Default|SetClosestInteractable (.ReturnValue (Actor|FindNearestActor (Transformation|GetActorLocation) (Variables|Default|GetInteractablesInInteract)))))))