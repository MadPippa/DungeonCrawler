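; Player bubble gun that blows bubble actors from an Arrow component aimed at the crosshair.
; Each tick, a visibility trace along the camera's forward vector turns the Arrow toward the hit point, or the trace end on a miss.
; BeginBubbleBlow spawns a PotionClass actor attached to the Arrow and starts it blowing.
; EndBubbleBlow detaches the bubble in world space, if still valid, and ends its blowing.
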(event Custom|BeginBubbleBlow
  (bind _returnvalue (Game|SpawnActorfromClass (Variables|Default|GetPotionClass) (Transformation|GetWorldTransform (Variables|Default|GetArrow)) "Undefined" "MultiplyWithRoot" 0 0))
  (bind _output_get (Variables|Default|SetBubble _returnvalue))
  (Transformation|AttachComponentToComponent _output_get (Variables|Default|GetArrow) "None" "SnapToTarget" "SnapToTarget" "SnapToTarget" true)
  (Default|BeginBlowing _output_get))

(event Custom|EndBubbleBlow
  (bind _bubble (Variables|Default|GetBubble)
    (:then
      (Transformation|DetachFromActor _bubble "KeepWorld" "KeepWorld" "KeepWorld")
      (Default|EndBlowing _bubble))
    (:else)))

(event EventBeginPlay)

(event Collision|EventActorBeginOverlap
  (params (OtherActor :type Actor%20Object%20Reference)))

(event EventTick
  (params (DeltaSeconds :type Float%20%28single-precision%29))
  (CallFunction|AimArrowtoCrosshair))

(fn ConstructionScript)

(fn AimArrowtoCrosshair
  (bind _returnvalue (Game|GetPlayerCameraManager 0))
  (bind _arrow (Variables|Default|GetArrow))
  (bind _transformcomponent (Variables|/Script/Engine.PlayerCameraManager|GetTransformComponent _returnvalue))
  (bind _returnvalue_2 (Transformation|GetWorldLocation _transformcomponent))
  (bind (_outhit _returnvalue_3) (Collision|LineTraceByChannel _returnvalue_2 (+ _returnvalue_2 (* (Math|Vector|GetForwardVector _transformcomponent) 1e+06)) "TraceTypeQuery1" false 0 "None"))
  (Transformation|SetWorldRotation _arrow (Math|Rotator|FindLookatRotation (Transformation|GetWorldLocation _arrow) (Math|Vector|SelectVector (.Location (Collision|BreakHitResult _outhit)) (.TraceEnd (Collision|BreakHitResult _outhit)) _returnvalue_3)) false false))