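; Actor component AC_Health tracks current and maximum health for its owning actor through Damage, Heal and Death events.
; Damage subtracts from CurrentHealth, or calls DeathMessage without changing it when the result would be zero or less.
; Heal adds health below the maximum, but otherwise assigns MaxHealth to itself, leaving CurrentHealth unchanged.
; Death destroys the owner and is not called directly within this graph.
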(event EventBeginPlay)

(event EventTick
  (params (DeltaSeconds :type Float%20%28single-precision%29)))

(event EventDamage
  (params (DamageAmount :type Float%20%28double-precision%29))
  (if (<= (- (Variables|Default|GetCurrentHealth) DamageAmount) 0.0)
    (Class|BIHealth|Death(Message) self)
    (else
      (Variables|Default|SetCurrentHealth (- (Variables|Default|GetCurrentHealth) DamageAmount)))))

(event EventHeal
  (params (HealAmount :type Float%20%28double-precision%29))
  (if (>= (+ HealAmount (Variables|Default|GetCurrentHealth)) (Variables|Default|GetMaxHealth))
    (Variables|Default|SetMaxHealth (Variables|Default|GetMaxHealth))
    (else
      (Variables|Default|SetCurrentHealth (+ HealAmount (Variables|Default|GetCurrentHealth))))))

(event EventDeath
  (Actor|DestroyActor (Components|GetOwner)))